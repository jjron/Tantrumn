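; EpicCharacter is the player character Blueprint for Tantrumn, handling the switch between normal follow and aiming modes.
; Tick detects changes in IsAiming, then snaps the follow camera between two marker locations and toggles controller-facing versus movement-facing rotation.
; A Hold macro separates Tap from Held using a retriggerable delay and two gates.
; Jump timing, distance and apex debug prints remain but are disconnected.
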(event `self.OnJumped`)

(event `self.OnLanded`
  (params (Hit :type "HitResult Structure (by ref)")))

(event `self.ReceiveTick`
  (params (DeltaSeconds :type "Float (single-precision)"))
  (bind _returnvalue (`self.IsAiming`))
  (if (!= _returnvalue (`self.bIsAiming`))
    (if _returnvalue
      (`self.OnStartAim`)
      (else
        (`self.OnStopAim`)))
    (set `self.bIsAiming` _returnvalue)))

(fn `OnStartAim`
  (bind _charactermovement (`self.CharacterMovement`))
  (`SceneComponent.K2_SetRelativeLocation` (`self.FollowCamera`) (`SceneComponent.RelativeLocation` (`self.AimCamLocation`)) false false)
  (set `CharacterMovementComponent.bUseControllerDesiredRotation` true _charactermovement)
  (set `CharacterMovementComponent.bOrientRotationToMovement` false _charactermovement))

(fn `OnStopAim`
  (bind _charactermovement (`self.CharacterMovement`))
  (`SceneComponent.K2_SetRelativeLocation` (`self.FollowCamera`) (`SceneComponent.RelativeLocation` (`self.FollowCamLocation`)) false false)
  (set `CharacterMovementComponent.bUseControllerDesiredRotation` false _charactermovement)
  (set `CharacterMovementComponent.bOrientRotationToMovement` true _charactermovement))

(fn `UserConstructionScript`)